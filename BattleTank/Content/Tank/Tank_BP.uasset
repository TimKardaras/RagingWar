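; Player tank Blueprint that binds driving, aiming and firing input to its components.
; BeginPlay passes barrel and turret to TankAiming and both tracks to TankMovement, which receive fire and move/turn input, while per-track throttle inputs drive tracks directly.
; Frame-time-scaled aim input rotates the azimuth gimbal and spring arm.
; Crosshair and reload widget logic is mostly disconnected; the live I key only hides the cursor and removes the never-assigned Reload widget.
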(event `Click`)

(event `self.ReceiveBeginPlay`
  (`TankAimingComponent.Initialise` (`self.TankAiming`) (`self.Barrel`) (`self.Turret`))
  (`TankMovementComponent.Initialise` (`self.TankMovement`) (`self.Left Track`) (`self.Right Track`)))

(event `Key|I`
  (params (Key :type "Key Structure" :default "AnyKey"))
  (bind _returnvalue (`GameplayStatics.GetPlayerController` 0))
  (:`Pressed`
    (if true
      (`/Engine/EditorBlueprintResources/StandardMacros.FlipFlop`
        (:`A`
          (set `PlayerController.bShowMouseCursor` false _returnvalue)
          (`Widget.RemoveFromParent` (`self.Reload`)))
        (:`B`
          (set `PlayerController.bShowMouseCursor` false _returnvalue))))))

(event `InputAction|Fire`
  (params (Key :type "Key Structure" :default "AnyKey")))

(event `InputAction|Fire`
  (params (Key :type "Key Structure" :default "AnyKey")))

(event `InputAxis|Turn Right`
  (params (AxisValue :type "Float (single-precision)"))
  ;[1 1 1] Comment
  (`TankMovementComponent.IntendTurnRight` (`self.TankMovement`) AxisValue))

(event `InputAxis|Turn Left`
  (params (AxisValue :type "Float (single-precision)"))
  ;[1 1 1] Comment
  (`TankMovementComponent.IntendTurnLeft` (`self.TankMovement`) AxisValue))

(event `InputAxis|Move Backward`
  (params (AxisValue :type "Float (single-precision)"))
  ;[1 1 1] Comment
  (`TankMovementComponent.IntendMoveBackward` (`self.TankMovement`) AxisValue))

(event `InputAxis|Move Forward`
  (params (AxisValue :type "Float (single-precision)"))
  ;[1 1 1] Comment
  (`TankMovementComponent.IntendMoveForward` (`self.TankMovement`) AxisValue))

(event `InputAxis|Right Track Throttle`
  (params (AxisValue :type "Float (single-precision)"))
  ;[1 1 1] Tank Movement Input Binding
  (`TankTrack.SetThrottle` (`self.Right Track`) AxisValue))

(event `InputAction|Fire`
  (params (Key :type "Key Structure" :default "AnyKey"))
  ;[1 1 1] Balistics
  (:`Pressed`
    (`TankAimingComponent.Fire` (`self.TankAiming`))))

(event `InputAxis|Left Track Throttle`
  (params (AxisValue :type "Float (single-precision)"))
  ;[1 1 1] Tank Movement Input Binding
  (`TankTrack.SetThrottle` (`self.Left Track`) AxisValue))

(event `InputAxis|AimAzimuth`
  (params (AxisValue :type "Float (single-precision)"))
  ;[1 1 1] Changes the Yaw Rotation of the spring arm by multiplying the axis value by the time
  ; of the last frame * 100
  (`SceneComponent.K2_AddLocalRotation` (`self.Azimuth Gimbal`) (`KismetMathLibrary.MakeRotator` 0.0 0.0 (* AxisValue (`GameplayStatics.GetWorldDeltaSeconds`) 100.0)) false false))

(event `InputAxis|AimElevation`
  (params (AxisValue :type "Float (single-precision)"))
  ;[1 1 1] Changes the Pitch elevation of the spring arm by multiplying the axis value by the time of the last frame * 100
  (`SceneComponent.K2_AddLocalRotation` (`self.SpringArm`) (`KismetMathLibrary.MakeRotator` 0.0 (* AxisValue (`GameplayStatics.GetWorldDeltaSeconds`) 100.0)) false false))

(fn `UserConstructionScript`)