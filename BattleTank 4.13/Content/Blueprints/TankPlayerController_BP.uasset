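; Player controller for a tank, handling the aiming HUD, pause menu and a placeholder vehicle exit.
; FoundAimingComponent creates the crosshair widget and passes it the aiming component reference.
; Pressing Pause shows the cursor and adds the pause menu; releasing it switches input to UI only.
; ExitVehicle only prints a message, and the death message and OnDeath widget chain is never run.
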(event `InputAction|ExitVehicle`
  (params (Key :type "Key Structure" :default "AnyKey"))
  (:`Pressed`
    (`KismetSystemLibrary.PrintString` "You Exit the Vehicle")))

(event `InputAction|Pause`
  (params (Key :type "Key Structure" :default "AnyKey"))
  ;[1 1 1] brings up the Pause Menu
  (:`Pressed`
    (set `self.bShowMouseCursor` true)
    (bind _returnvalue (`|CreateWidget` "/Game/Widgets/PauseMenu.PauseMenu_C"))
    (`UserWidget.AddToViewport` _returnvalue 0))
  (:`Released`
    (`WidgetBlueprintLibrary.SetInputMode_UIOnlyEx` (`GameplayStatics.GetPlayerController` 0))))

(event `self.FoundAimingComponent`
  (params (AimCompRef :type "TankAimingComponent Object Reference"))
  ;[1 1 1] Creating a crosshair widget because the Player Crosshair is a BP widget,
  ; we then add it to the viewport and also adding the UI
  (bind _returnvalue (`|CreateWidget` "/Game/Widgets/PlayerCrosshair.PlayerCrosshair_C"))
  (`UserWidget.AddToViewport` _returnvalue 0)
  (set `/Game/Widgets/PlayerCrosshair.BP Aiming Comp. Reference` AimCompRef _returnvalue))

(fn `UserConstructionScript`)